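; Player pawn with enhanced-input movement and look, weapon toggling and aimed hitscan shooting.
; It creates the MainUI widget, shows the crosshair while aiming, and toggles weapons through BP_Controller when not manning and gunning is allowed.
; Shots trace from the camera with random spread, damage Evil actors and record hit direction, then drain controller ammo behind a short fire cooldown.
; Debug drawing is active for aiming and shots.
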(event Input|EnhancedActionEvents|EnhancedInputActionIA_GunningToggle
  (params (ActionValue :type Boolean) (ElapsedSeconds :type Float%20%28double-precision%29) (TriggeredSeconds :type Float%20%28double-precision%29) (InputAction :type Input%20Action%20Object%20Reference :default "/Game/Blueprints/Player/IA_GunningToggle.IA_GunningToggle"))
  (bind _asbp_standered (Utilities|Casting|CastToBP_Controller (Pawn|GetController)))
  (if (and (not (Variables|/Game/Blueprints/Player/BP_Controller.BP_Controller_C|GetManning _asbp_standered)) (Variables|Default|GetCanGun))
    (Default|ToggleWeapon _asbp_standered)))

(event Input|EnhancedActionEvents|EnhancedInputActionIA_Shoot
  (params (ActionValue :type Boolean) (ElapsedSeconds :type Float%20%28double-precision%29) (TriggeredSeconds :type Float%20%28double-precision%29) (InputAction :type Input%20Action%20Object%20Reference :default "/Game/Blueprints/Player/IA_Shoot.IA_Shoot"))
  (bind _random_spread (Variables|Default|GetRandom%20Spread))
  (bind _camera (Variables|Default|GetCamera))
  (bind _returnvalue (Transformation|GetWorldLocation _camera))
  (bind _returnvalue_2 (* _random_spread -1.0))
  (if (and (Variables|Default|Getcanfire) (Variables|Default|GetAiming))
    (Variables|Default|Setcanfire false)
    (bind (_outhit _returnvalue_3) (Collision|LineTraceByChannel _returnvalue (Math|Vector|RotateVector (+ _returnvalue (Math|Vector|MakeVector 9e+05 (Math|Random|RandomFloatinRange _returnvalue_2 _random_spread) (Math|Random|RandomFloatinRange _returnvalue_2 _random_spread))) (Transformation|GetWorldRotation _camera)) "TraceTypeQuery3" false 0 "ForDuration" true "(R=1.000000,G=0.412919,B=0.000000,A=1.000000)" "(R=0.000000,G=1.000000,B=0.000000,A=1.000000)" 1.0))
    (if _returnvalue_3
      (bind _asevil (Utilities|Casting|CastToEvil (.HitActor (Collision|BreakHitResult _outhit)))
        (:then
          (Utilities|FlowControl|Sequence
            (:then_0
              (Default|TakeDamage _asevil (Variables|Default|GetDamage))
              (Variables|/Game/Blueprints/Enemies/Evil.Evil_C|SetHitThing _asevil (Math|Rotator|FindLookatRotation (Transformation|GetActorLocation) (.Location (Collision|BreakHitResult _outhit)))))
            (:then_1
              (Default|DrainAmmo (Variables|Default|GetAs%20BP%20Standered) -1 :!label _label)
              (Utilities|FlowControl|Delay 0.1)
              (Variables|Default|Setcanfire true))))
        (:CastFailed
          (goto _label)))
      (else
        (goto _label)))))

(event Input|EnhancedActionEvents|EnhancedInputActionIA_LeftRight
  (params (ActionValue :type Float%20%28double-precision%29) (ElapsedSeconds :type Float%20%28double-precision%29) (TriggeredSeconds :type Float%20%28double-precision%29) (InputAction :type Input%20Action%20Object%20Reference :default "/Game/Blueprints/Player/IA_LeftRight.IA_LeftRight"))
  ;[0 0 1] Player Movement
  (Pawn|Input|AddMovementInput (Math|Vector|RotateVector (Math|Vector|MakeVector 0.0 ActionValue 0.0) (Math|Rotator|MakeRotator 0.0 0.0 (.yaw (Transformation|GetWorldRotation (Variables|Collision|GetCapsuleComponent))))) 1.0 false))

(event Input|EnhancedActionEvents|EnhancedInputActionIA_Look
  (params (ActionValue :type Vector%202D%20Structure) (ElapsedSeconds :type Float%20%28double-precision%29) (TriggeredSeconds :type Float%20%28double-precision%29) (InputAction :type Input%20Action%20Object%20Reference :default "/Game/Blueprints/Player/IA_Look.IA_Look"))
  ;[0 0 1] Player Movement
  (Pawn|Input|AddControllerYawInput (.x ActionValue))
  (Pawn|Input|AddControllerPitchInput (* (.y ActionValue) -1.0)))

(event Input|EnhancedActionEvents|EnhancedInputActionIA_Ads
  (params (ActionValue :type Boolean) (ElapsedSeconds :type Float%20%28double-precision%29) (TriggeredSeconds :type Float%20%28double-precision%29) (InputAction :type Input%20Action%20Object%20Reference :default "/Game/Blueprints/Player/IA_Ads.IA_Ads"))
  (bind _ui (Variables|Default|GetUI))
  (bind _capsulecomponent (Variables|Collision|GetCapsuleComponent))
  (bind _returnvalue (Transformation|GetWorldLocation _capsulecomponent))
  (bind _crossair (Variables|/Game/Blueprints/UI/MainUI.MainUI_C|GetCrossair _ui))
  (:Triggered
    (Variables|Default|SetAiming true)
    (Variables|/Script/UMG.Widget|SetVisibility _crossair "Visible")
    (Rendering|Debug|DrawDebugArrow _returnvalue (Math|Vector|RotateVector (+ _returnvalue (Math|Vector|RotateVector "150.000000,0.000000,0.000000" (Transformation|GetWorldRotation _capsulecomponent))) "0, 0, 0") 0.0 "(R=1.000000,G=0.000000,B=0.000000,A=1.000000)" 0.0 1.0))
  (:Completed
    (Variables|Default|SetAiming false)
    (Variables|/Script/UMG.Widget|SetVisibility _crossair "Hidden")))

(event Input|EnhancedActionEvents|EnhancedInputActionIA_ForwardBack
  (params (ActionValue :type Float%20%28double-precision%29) (ElapsedSeconds :type Float%20%28double-precision%29) (TriggeredSeconds :type Float%20%28double-precision%29) (InputAction :type Input%20Action%20Object%20Reference :default "/Game/Blueprints/Player/IA_ForwardBack.IA_ForwardBack"))
  ;[0 0 1] Player Movement
  (Pawn|Input|AddMovementInput (Math|Vector|RotateVector (Math|Vector|MakeVector ActionValue 0.0 0.0) (Math|Rotator|MakeRotator 0.0 0.0 (.yaw (Transformation|GetWorldRotation (Variables|Collision|GetCapsuleComponent))))) 1.0 false))

(event EventBeginPlay
  (bind _asbp_standered (Utilities|Casting|CastToBP_Controller (Pawn|GetController)))
  (bind _returnvalue (UserInterface|CreateWidget "/Game/Blueprints/UI/MainUI.MainUI_C" _asbp_standered))
  (Variables|Default|SetUI _returnvalue)
  (Variables|/Script/UMG.Widget|SetVisibility (Variables|/Game/Blueprints/UI/MainUI.MainUI_C|GetCrossair _returnvalue) "Hidden")
  (Variables|/Script/UMG.Widget|SetVisibility (Variables|/Game/Blueprints/UI/MainUI.MainUI_C|GetTextBlock_0 _returnvalue) "Hidden")
  (UserInterface|Viewport|AddtoViewport _returnvalue 0))

(event EventPossessed
  (params (NewController :type Controller%20Object%20Reference))
  (bind _asbp_standered (Utilities|Casting|CastToBP_Controller NewController))
  (Variables|Default|SetAs%20BP%20Standered _asbp_standered))

(fn ConstructionScript)