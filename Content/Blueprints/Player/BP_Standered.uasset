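; BP_Standered is a player controller that switches control between the player pawn and a gun that the player mans.
; On BeginPlay it adds the standard input mapping context.
; ToggleWeapon flip-flops between standard and gun contexts, possessing BP_Gun or BP_Player found by class and recording the state in Manning.
; Gun mode also hides a player UI text block and shows a crosshair widget as the mouse cursor.
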(event Custom|ToggleWeapon
  (bind _returnvalue (PlayerController|LocalPlayerSubsystems|GetEnhancedInputLocalPlayerSubsystem))
  (bind _isa (Utilities|FlowControl|FlipFlop)
    (:A
      (Input|AddMappingContext _returnvalue "/Game/Blueprints/Player/IM_Gun.IM_Gun" 0 "(bIgnoreAllPressedKeysUntilRelease=True,bForceImmediately=False,bNotifyUserSettings=False)")
      (Input|RemoveMappingContext _returnvalue "/Game/Blueprints/Player/IM_Standard.IM_Standard" "(bIgnoreAllPressedKeysUntilRelease=True,bForceImmediately=False,bNotifyUserSettings=False)")
      (bind _returnvalue_2 (Actor|GetActorOfClass "/Game/Blueprints/Player/BP_Gun.BP_Gun_C"))
      (bind _returnvalue_3 (Actor|GetActorOfClass "/Game/Blueprints/Player/BP_Player.BP_Player_C"))
      (Pawn|UnPossess)
      (Pawn|Possess _returnvalue_2)
      (Variables|/Script/UMG.Widget|SetVisibility (Variables|/Game/Blueprints/UI/MainUI.MainUI_C|GetTextBlock_0 (Variables|/Game/Blueprints/Player/BP_Player.BP_Player_C|GetUI _returnvalue_3)) "Hidden")
      (Variables|Default|SetbShowMouseCursor true)
      (bind _returnvalue_4 (UserInterface|CreateWidget "/Game/Blueprints/UI/Crossair.Crossair_C"))
      (Class|PlayerController|SetMouseCursorWidget "Default" _returnvalue_4))
    (:B
      (Input|AddMappingContext _returnvalue "/Game/Blueprints/Player/IM_Standard.IM_Standard" 0 "(bIgnoreAllPressedKeysUntilRelease=True,bForceImmediately=False,bNotifyUserSettings=False)")
      (Input|RemoveMappingContext _returnvalue "/Game/Blueprints/Player/IM_Gun.IM_Gun" "(bIgnoreAllPressedKeysUntilRelease=True,bForceImmediately=False,bNotifyUserSettings=False)")
      (bind _returnvalue_5 (Actor|GetActorOfClass "/Game/Blueprints/Player/BP_Player.BP_Player_C"))
      (Pawn|UnPossess)
      (Pawn|Possess _returnvalue_5)
      (Variables|/Script/UMG.Widget|SetVisibility (Variables|/Game/Blueprints/UI/MainUI.MainUI_C|GetTextBlock_0 (Variables|/Game/Blueprints/Player/BP_Player.BP_Player_C|GetUI _returnvalue_5)) "Visible")
      (Variables|Default|SetbShowMouseCursor false)))
  (Variables|Default|SetManning _isa))

(event EventBeginPlay
  (Input|AddMappingContext (PlayerController|LocalPlayerSubsystems|GetEnhancedInputLocalPlayerSubsystem) "/Game/Blueprints/Player/IM_Standard.IM_Standard" 0 "(bIgnoreAllPressedKeysUntilRelease=True,bForceImmediately=False,bNotifyUserSettings=False)"))

(fn ConstructionScript)