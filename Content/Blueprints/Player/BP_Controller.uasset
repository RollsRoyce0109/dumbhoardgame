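; Player controller that lets the player switch between controlling BP_Player and manning that player's weapon.
; ToggleWeapon flip-flops possession between the two, swaps the standard and gun Enhanced Input contexts, and records the state in Manning.
; Manning the weapon shows a crosshair cursor and hides a player UI text block; leaving restores the text and hides the cursor.
; DrainAmmo and GetMoney add the passed amount to Ammunition and Money, then print the result.
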(event Custom|Drain%20Ammo
  (params (Cost :type Integer))
  (bind _ammunition (Variables|Default|GetAmmunition))
  (bind _result (Utilities|ManipulateIntInternal _ammunition (+ _ammunition Cost))
    (:%20%20
      (Development|PrintString (Utilities|String|ToString(Integer) _result)))))

(event Custom|ToggleWeapon
  (bind _returnvalue (PlayerController|LocalPlayerSubsystems|GetEnhancedInputLocalPlayerSubsystem))
  (bind _isa (Utilities|FlowControl|FlipFlop)
    (:A
      (Input|AddMappingContext _returnvalue "/Game/Blueprints/Player/IM_Gun.IM_Gun" 0 "(bIgnoreAllPressedKeysUntilRelease=True,bForceImmediately=False,bNotifyUserSettings=False)")
      (Input|RemoveMappingContext _returnvalue "/Game/Blueprints/Player/IM_Standard.IM_Standard" "(bIgnoreAllPressedKeysUntilRelease=True,bForceImmediately=False,bNotifyUserSettings=False)")
      (bind _returnvalue_2 (Actor|GetActorOfClass "/Game/Blueprints/Player/BP_Player.BP_Player_C"))
      (Pawn|UnPossess)
      (Pawn|Possess (Variables|/Game/Blueprints/Player/BP_Player.BP_Player_C|GetThineWeapon _returnvalue_2))
      (Variables|/Script/UMG.Widget|SetVisibility (Variables|/Game/Blueprints/UI/MainUI.MainUI_C|GetTextBlock_0 (Variables|/Game/Blueprints/Player/BP_Player.BP_Player_C|GetUI _returnvalue_2)) "Hidden")
      (Variables|Default|SetbShowMouseCursor true)
      (bind _returnvalue_3 (UserInterface|CreateWidget "/Game/Blueprints/UI/Crossair.Crossair_C"))
      (Class|PlayerController|SetMouseCursorWidget "Default" _returnvalue_3))
    (:B
      (Input|AddMappingContext _returnvalue "/Game/Blueprints/Player/IM_Standard.IM_Standard" 0 "(bIgnoreAllPressedKeysUntilRelease=True,bForceImmediately=False,bNotifyUserSettings=False)")
      (Input|RemoveMappingContext _returnvalue "/Game/Blueprints/Player/IM_Gun.IM_Gun" "(bIgnoreAllPressedKeysUntilRelease=True,bForceImmediately=False,bNotifyUserSettings=False)")
      (bind _returnvalue_4 (Actor|GetActorOfClass "/Game/Blueprints/Player/BP_Player.BP_Player_C"))
      (Pawn|UnPossess)
      (Pawn|Possess _returnvalue_4)
      (Variables|/Script/UMG.Widget|SetVisibility (Variables|/Game/Blueprints/UI/MainUI.MainUI_C|GetTextBlock_0 (Variables|/Game/Blueprints/Player/BP_Player.BP_Player_C|GetUI _returnvalue_4)) "Visible")
      (Variables|Default|SetbShowMouseCursor false)))
  (Variables|Default|SetManning _isa))

(event EventBeginPlay
  (Input|AddMappingContext (PlayerController|LocalPlayerSubsystems|GetEnhancedInputLocalPlayerSubsystem) "/Game/Blueprints/Player/IM_Standard.IM_Standard" 0 "(bIgnoreAllPressedKeysUntilRelease=True,bForceImmediately=False,bNotifyUserSettings=False)"))

(fn ConstructionScript)

(fn GetMoney
  (params (Money :type Float%20%28double-precision%29))
  (bind _result (Utilities|ManipulateFloatInternal (Variables|Default|GetMoney) (+ (Variables|Default|GetMoney) Money))
    (:%20%20
      (Development|PrintString (Utilities|String|ToString(Float) _result)))))