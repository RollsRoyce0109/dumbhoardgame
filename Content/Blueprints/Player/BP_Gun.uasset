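; BP_Gun is a mountable gun that the player can man and fire with the mouse.
; Overlap flags BP_Player as able to gun and shows a UI prompt, while the toggle input asks BP_Controller to switch out when manning.
; Shooting traces from the cursor's world position with random spread, damages Evil actors and passes them the hit direction.
; Each shot drains ammo through the possessing controller, with a short delay gating fire rate.
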(event Input|EnhancedActionEvents|EnhancedInputActionIA_GunningToggle
  (params (ActionValue :type Boolean) (ElapsedSeconds :type Float%20%28double-precision%29) (TriggeredSeconds :type Float%20%28double-precision%29) (InputAction :type Input%20Action%20Object%20Reference :default "/Game/Blueprints/Player/IA_GunningToggle.IA_GunningToggle"))
  (bind _asbp_standered (Utilities|Casting|CastToBP_Controller (Pawn|GetController)))
  (if (Variables|/Game/Blueprints/Player/BP_Controller.BP_Controller_C|GetManning _asbp_standered)
    (Default|ToggleWeapon _asbp_standered)))

(event Input|EnhancedActionEvents|EnhancedInputActionIA_Shoot
  (params (ActionValue :type Boolean) (ElapsedSeconds :type Float%20%28double-precision%29) (TriggeredSeconds :type Float%20%28double-precision%29) (InputAction :type Input%20Action%20Object%20Reference :default "/Game/Blueprints/Player/IA_Shoot.IA_Shoot"))
  (bind _returnvalue (Game|GetPlayerController 0))
  (bind _random_spread (Variables|Default|GetRandom%20Spread))
  (bind (_worldlocation _worlddirection) (Game|Player|ConvertMouseLocationToWorldSpace _returnvalue))
  (bind _returnvalue_2 (* _random_spread -1.0))
  (if (Variables|Default|Getcanfire)
    (Variables|Default|Setcanfire false)
    (bind (_outhit _returnvalue_3) (Collision|LineTraceByChannel _worldlocation (Math|Vector|RotateVector (+ _worldlocation (Math|Vector|MakeVector 9e+05 (Math|Random|RandomFloatinRange _returnvalue_2 _random_spread) (Math|Random|RandomFloatinRange _returnvalue_2 _random_spread))) (Math|Conversions|RotationFromXVector _worlddirection)) "TraceTypeQuery3" false 0 "ForDuration" true "(R=1.000000,G=0.000000,B=0.000000,A=1.000000)" "(R=0.000000,G=1.000000,B=0.000000,A=1.000000)" 1.0))
    (if _returnvalue_3
      (bind _asevil (Utilities|Casting|CastToEvil (.HitActor (Collision|BreakHitResult _outhit)))
        (:then
          (Utilities|FlowControl|Sequence
            (:then_0
              (Default|TakeDamage _asevil (Variables|Default|GetDamage))
              (Variables|/Game/Blueprints/Enemies/Evil.Evil_C|SetHitThing _asevil (Math|Rotator|FindLookatRotation (Transformation|GetActorLocation) (.Location (Collision|BreakHitResult _outhit)))))
            (:then_1
              (Default|DrainAmmo (Variables|Default|GetAs%20BP%20Standered) -1 :!label _label)
              (Utilities|FlowControl|Delay 0.2)
              (Variables|Default|Setcanfire true))))
        (:CastFailed
          (goto _label)))
      (else
        (goto _label)))))

(event EventPossessed
  (params (NewController :type Controller%20Object%20Reference))
  (bind _asbp_standered (Utilities|Casting|CastToBP_Controller NewController))
  (Variables|Default|SetAs%20BP%20Standered _asbp_standered))

(event Collision|EventActorBeginOverlap
  (params (OtherActor :type Actor%20Object%20Reference))
  (bind _asbp_player (Utilities|Casting|CastToBP_Player OtherActor))
  (Variables|/Game/Blueprints/Player/BP_Player.BP_Player_C|SetCanGun _asbp_player true)
  (Variables|/Game/Blueprints/Player/BP_Player.BP_Player_C|SetThineWeapon _asbp_player self)
  (Variables|/Script/UMG.Widget|SetVisibility (Variables|/Game/Blueprints/UI/MainUI.MainUI_C|GetTextBlock_0 (Variables|/Game/Blueprints/Player/BP_Player.BP_Player_C|GetUI _asbp_player)) "Visible"))

(event Collision|EventActorEndOverlap
  (params (OtherActor :type Actor%20Object%20Reference))
  (bind _asbp_player (Utilities|Casting|CastToBP_Player OtherActor))
  (Variables|/Game/Blueprints/Player/BP_Player.BP_Player_C|SetCanGun _asbp_player false)
  (Variables|/Game/Blueprints/Player/BP_Player.BP_Player_C|SetThineWeapon _asbp_player 0)
  (Variables|/Script/UMG.Widget|SetVisibility (Variables|/Game/Blueprints/UI/MainUI.MainUI_C|GetTextBlock_0 (Variables|/Game/Blueprints/Player/BP_Player.BP_Player_C|GetUI _asbp_player)) "Hidden"))

(fn ConstructionScript)