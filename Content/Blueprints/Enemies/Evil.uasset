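; Enemy actor that advances on BP_Gun, takes damage and pays the player random money on death.
; Five seconds after BeginPlay, a looping timer teleport-steps it toward the gun; a downward trace hit bumps it upward and re-aims it.
; TakeDamage adds a signed amount to Health and briefly swaps the cube's material.
; Death stops movement, launches the capsule with an impulse, credits BP_Controller and destroys the actor after a delay.
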(event Custom|Begin%20delete
  (Utilities|FlowControl|DelayUntilNextTick)
  (Collision|SetCollisionEnabled (Variables|Default|GetCapsule) "PhysicsOnly")
  (Utilities|FlowControl|Delay 1.5)
  (Actor|DestroyActor))

(event Custom|BeginMoving
  (bind _returnvalue (Utilities|Time|SetTimerbyEvent (delegate Custom|Move) 0.05 true))
  (Variables|Default|SetMovement _returnvalue)
  (bind _returnvalue_2 (Actor|GetActorOfClass "/Game/Blueprints/Player/BP_Gun.BP_Gun_C"))
  (Transformation|SetActorRotation (Math|Rotator|FindLookatRotation (Transformation|GetActorLocation) (Transformation|GetActorLocation _returnvalue_2)) true))

(event Custom|Move
  (bind _emptyscenecomponent (Variables|Default|GetEmptySceneComponent))
  (bind _returnvalue (Transformation|GetWorldLocation _emptyscenecomponent))
  (bind (_x _y _z) (Math|Vector|BreakVector _returnvalue))
  (Utilities|FlowControl|Sequence
    (:then_0
      (bind _returnvalue_2 (Collision|LineTraceByChannel _returnvalue (Math|Vector|MakeVector _x _y (- _z 8e+01)) "TraceTypeQuery1" false 0 "None"))
      (if _returnvalue_2
        (Development|PrintString "Hello")
        (Transformation|SetActorLocation (Math|Vector|MakeVector _x _y (+ _z 1e+02)) false true)
        (bind _returnvalue_3 (Actor|GetActorOfClass "/Game/Blueprints/Player/BP_Gun.BP_Gun_C"))
        (Transformation|SetActorRotation (Math|Rotator|FindLookatRotation (Transformation|GetActorLocation) (Transformation|GetActorLocation _returnvalue_3)) true)))
    (:then_1
      (Transformation|SetActorLocation self (+ (Transformation|GetActorLocation) (Math|Vector|RotateVector (* (Class|KismetMathLibrary|VectorForward) (Math|Float|MakeLiteralFloat 5.0)) (Math|Rotator|FindLookatRotation (Transformation|GetActorLocation) (Transformation|GetActorLocation (stale Custom|BeginMoving _returnvalue_2))))) false true))))

(event EventBeginPlay
  (CallFunction|EnemySetup)
  (Utilities|FlowControl|Delay 5.0)
  (CallFunction|BeginMoving))

(fn ConstructionScript)

(fn TakeDamage
  (params (ToTake :type Float%20%28double-precision%29))
  (Rendering|Material|SetMaterial (Variables|Default|GetCube) 0 "/Game/Blueprints/Enemies/NewMaterial1.NewMaterial1")
  (bind _output_get (Variables|Default|SetHealth (+ (Variables|Default|GetHealth) ToTake)))
  (Development|PrintString (Utilities|String|ToString(Float) _output_get))
  (if (and (<= (Variables|Default|GetHealth) 0.0) (Variables|Default|GetAlive))
    (CallFunction|Death)
    (else
      (Utilities|Time|SetTimerbyFunctionName 0 "Unhurt" 0.1))))

(fn EnemySetup
  (Variables|Default|SetHealth (Variables|Default|GetMaximumHealth)))

(fn Death
  (Utilities|Time|ClearandInvalidateTimerbyHandle (Variables|Default|GetMovement))
  (Class|PrimitiveComponent|SetConstraintMode (Variables|Default|GetCapsule) "None")
  (Variables|Default|SetAlive false)
  (Development|PrintString "gaaah")
  (Collision|SetCollisionResponsetoChannel (Variables|Default|GetCapsule) "ECC_GameTraceChannel1" "ECR_Ignore")
  (Physics|AddImpulse (Variables|Default|GetCapsule) (Math|Vector|RotateVector (Math|Vector|MakeVector 1e+03 0.0 5e+02) (Variables|Default|GetHitThing)) "None" true)
  (bind _asbp_standered (Utilities|Casting|CastToBP_Controller (Game|GetPlayerController 0)))
  (Default|GetMoney _asbp_standered (/ (Math|Conversions|ToFloat(Integer) (Math|Float|Round (Math|Random|RandomFloatinRange 2.5e+02 3e+02))) 1e+02))
  (CallFunction|BeginDelete))

(fn Unhurt
  (Rendering|Material|SetMaterial (Variables|Default|GetCube) 0 "/Game/Blueprints/Enemies/NewMaterial.NewMaterial"))