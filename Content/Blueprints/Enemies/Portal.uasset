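; Portal is an enemy spawner actor that periodically spawns Evil enemies aimed at the BP_Gun actor.
; A looping timer started at BeginPlay spawns an Evil at an offset from the portal, skipping the spawn if that spot would collide.
; After a one-tick delay, a valid spawn is rotated from the spawn point toward the gun's location and told to begin moving.
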(event Custom|spawn%20evils
  (bind _returnvalue (Transformation|GetActorLocation))
  (bind _newvar (Variables|Default|GetNewVar))
  (bind _returnvalue_2 (+ _returnvalue _newvar))
  (bind _returnvalue_3 (Game|SpawnActorfromClass "/Game/Blueprints/Enemies/Evil.Evil_C" (Math|Transform|MakeTransform _returnvalue_2 "0, 0, 0" "1.000000,1.000000,1.000000") "DontSpawnIfColliding" "MultiplyWithRoot" 0 0.0 2e+01 0))
  (Utilities|FlowControl|DelayUntilNextTick)
  (Utilities|IsValid _returnvalue_3
    (:Is%20Valid
      (bind _returnvalue_4 (Actor|GetActorOfClass "/Game/Blueprints/Player/BP_Gun.BP_Gun_C"))
      (Transformation|SetActorRotation _returnvalue_3 (Math|Rotator|FindLookatRotation _returnvalue_2 (Transformation|GetActorLocation _returnvalue_4)) true)
      (Default|BeginMoving _returnvalue_3))))

(event EventBeginPlay
  (Utilities|Time|SetTimerbyEvent (delegate Custom|spawn%20evils) 5.0 true))

(fn ConstructionScript)