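; Portal actor that spawns an Evil enemy and launches it toward the BP_Gun actor.
; A timer started on BeginPlay triggers the spawn at an offset from the portal's location.
; One tick after spawning, it rotates the enemy to face the gun and calls its Move with a vector pointing in that direction.
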(event Custom|spawn%20evils
  (bind _returnvalue (Transformation|GetActorLocation))
  (bind _newvar (Variables|Default|GetNewVar))
  (bind _returnvalue_2 (+ _returnvalue _newvar))
  (bind _returnvalue_3 (Game|SpawnActorfromClass "/Game/Blueprints/Enemies/Evil.Evil_C" (Math|Transform|MakeTransform _returnvalue_2 "0, 0, 0" "1.000000,1.000000,1.000000") "Undefined" "MultiplyWithRoot" 0 0.0 2e+01 0))
  (Utilities|FlowControl|DelayUntilNextTick)
  (bind _returnvalue_4 (Actor|GetActorOfClass "/Game/Blueprints/Player/BP_Gun.BP_Gun_C"))
  (Transformation|SetActorRotation _returnvalue_3 (Math|Rotator|FindLookatRotation _returnvalue_2 (Transformation|GetActorLocation _returnvalue_4)))
  (Default|Move _returnvalue_3 (Math|Vector|RotateVector "1000.000000,0.000000,0.000000" (Math|Rotator|FindLookatRotation _returnvalue_2 (Transformation|GetActorLocation _returnvalue_4)))))

(event EventBeginPlay
  (Utilities|Time|SetTimerbyEvent (delegate Custom|spawn%20evils) 5.0))

(event Collision|EventActorBeginOverlap
  (params (OtherActor :type Actor%20Object%20Reference)))

(event EventTick
  (params (DeltaSeconds :type Float%20%28single-precision%29)))

(fn ConstructionScript)